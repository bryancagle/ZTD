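; The player's base in the ZTD game, an actor whose loss of all health ends the game.
; TakeDamage lowers Health and plays a hit sound at the game instance's sound level.
; Each tick, TestHealth copies Health to ZTD_Instance and, at zero, disables player input, blends the camera to the base and sets IsGameOver.
; While game over is set, Tick also runs a delayed particle activation and deactivation.
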(event `self.ReceiveTick`
  (params (DeltaSeconds :type "Float (single-precision)"))
  (bind _particlesystem (`self.ParticleSystem`))
  (`|ExecutionSequence`
    (:`then_0`
      ;[1 1 1] Tests if the base's health is 0, if it is thenyou lose
      (`self.TestHealth`))
    (:`then_1`
      (bind _asztd_instance (cast `/Game/ZTD_Blueprint/Blueprints/ZTD_Instance` (`GameplayStatics.GetGameInstance`)))
      (if (`/Game/ZTD_Blueprint/Blueprints/ZTD_Instance.IsGameOver` _asztd_instance)
        (`KismetSystemLibrary.Delay` 1.0)
        (`ActorComponent.Activate` _particlesystem false)
        (`KismetSystemLibrary.Delay` 0.5)
        (`ActorComponent.Deactivate` _particlesystem)))))

(event `TakeDamage`
  (params (Damage :type "Float (double-precision)"))
  (set `self.Health` (- (`self.Health`) Damage))
  (bind _asztd_instance (cast `/Game/ZTD_Blueprint/Blueprints/ZTD_Instance` (`GameplayStatics.GetGameInstance`)))
  (`GameplayStatics.PlaySound2D` "/Game/ZTD_Blueprint/Sounds/BASEHIT.BASEHIT" (`/Game/ZTD_Blueprint/Blueprints/ZTD_Instance.SoundLevel` _asztd_instance)))

(fn `TestHealth`
  (bind _returnvalue (`GameplayStatics.GetPlayerController` 0))
  (bind _health (`self.Health`))
  (bind _asztd_instance (cast `/Game/ZTD_Blueprint/Blueprints/ZTD_Instance` (`GameplayStatics.GetGameInstance`)))
  (set `/Game/ZTD_Blueprint/Blueprints/ZTD_Instance.CurrentBaseHealth` _health _asztd_instance)
  (if (<= _health 0.0)
    (`self.DisableInput` _returnvalue null)
    (`PlayerController.SetViewTargetWithBlend` _returnvalue self 1.0 "VTBlend_Linear" 0.0 false)
    (set `/Game/ZTD_Blueprint/Blueprints/ZTD_Instance.IsGameOver` true _asztd_instance)))

(fn `UserConstructionScript`)