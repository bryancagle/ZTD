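; Player character Blueprint that manages a two-level spring-arm camera zoom and triggers game over when health runs out.
; Zoom input actions set a target distance, which Tick eases the arm toward with FInterpTo using a fixed delta, so smoothing is frame-rate dependent.
; Tick also polls health; at zero or below it disables controller input, plays a sound at the game instance's volume and flags game over there, with no once-only guard.
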(event `self.ReceiveBeginPlay`
  ;[1 1 1] Activates camera - This was original VR related, I don't think it affects anything
  (`ActorComponent.Activate` (`self.Camera1`) false))

(event `self.ReceiveTick`
  (params (DeltaSeconds :type "Float (single-precision)"))
  (`|ExecutionSequence`
    (:`then_0`
      ;[1 1 1] Sets the spring arm to interp (smooth transition) to the selected camera zoom level
      (`self.InterpCameraDistance`))
    (:`then_1`
      ;[1 1 1] Tests if player's health is 0, in which you lose
      (`self.TestPlayerHealth`))))

(event `InputAction|ZoomOutCamera`
  (params (Key :type "Key Structure" :default "AnyKey"))
  ;[1 1 1] The controller input event to set the camera zoom
  (:`Pressed`
    (set `self.CameraZoom` 4500.0)))

(event `InputAction|ZoomInCamera`
  (params (Key :type "Key Structure" :default "AnyKey"))
  ;[1 1 1] The controller input event to set the camera zoom
  (:`Pressed`
    (set `self.CameraZoom` 2200.0)))

(fn `InterpCameraDistance`
  (bind _springarm1 (`self.SpringArm1`))
  (set `SpringArmComponent.TargetArmLength` (`KismetMathLibrary.FInterpTo` (`SpringArmComponent.TargetArmLength` _springarm1) (`self.CameraZoom`) 0.1 0.5) _springarm1))

(fn `TestPlayerHealth`
  (if (<= (`self.Health`) 0.0)
    (bind _asplayer_controller (cast `/Game/ZTD_Blueprint/Blueprints/Player_Controller` (`GameplayStatics.GetPlayerController` 0)))
    (`self.DisableInput` _asplayer_controller null)
    (bind _asztd_instance (cast `/Game/ZTD_Blueprint/Blueprints/ZTD_Instance` (`GameplayStatics.GetGameInstance`)))
    (`GameplayStatics.PlaySound2D` "/Game/StarterContent/Audio/Smoke01.Smoke01" (`/Game/ZTD_Blueprint/Blueprints/ZTD_Instance.SoundLevel` _asztd_instance) 0.0)
    (set `/Game/ZTD_Blueprint/Blueprints/ZTD_Instance.IsGameOver` true _asztd_instance)))

(fn `UserConstructionScript`)