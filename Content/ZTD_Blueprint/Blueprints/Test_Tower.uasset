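; Test tower actor that players buy and sell by clicking during tower placement mode.
; Tick shows its three meshes while placement mode is on or the tower is active, and hides them otherwise.
; Clicking any mesh buys it if ZTD_Instance currency suffices, switching to a solid material, or sells an active tower for a partial refund.
; Selling restores transparency and calls ChangeTower on all Tower_Tile actors.
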(event `self.ReceiveTick`
  (params (DeltaSeconds :type "Float (single-precision)"))
  ;[1 1 1] Unpurchased towers are shown or hidden when in placement mode or shooting
  (bind _asztd_instance (cast `/Game/ZTD_Blueprint/Blueprints/ZTD_Instance` (`GameplayStatics.GetGameInstance`)))
  (if (`/Game/ZTD_Blueprint/Blueprints/ZTD_Instance.IsTowerPlacement` _asztd_instance)
    (`SceneComponent.SetVisibility` (`self.TowerBody`) true false :!label _label)
    (`SceneComponent.SetVisibility` (`self.Sphere`) true false)
    (`SceneComponent.SetVisibility` (`self.Cylinder`) true false)
    (elif (`self.TowerActive`)
      (goto _label)
      (else
        (`SceneComponent.SetVisibility` (`self.TowerBody`) false false)
        (`SceneComponent.SetVisibility` (`self.Sphere`) false false)
        (`SceneComponent.SetVisibility` (`self.Cylinder`) false false)))))

(event `self.TowerBody.OnClicked`
  (params (TouchedComponent :type "PrimitiveComponent Object Reference") (ButtonPressed :type "Key Structure" :default "AnyKey"))
  ;[1 1 1] When towers are purchased, they are set to a solid material and decrease currency. When sold they increase currency and set to transparent again
  (bind _asztd_instance (cast `/Game/ZTD_Blueprint/Blueprints/ZTD_Instance` (`GameplayStatics.GetGameInstance`) :!label _label_2))
  (if (`/Game/ZTD_Blueprint/Blueprints/ZTD_Instance.IsTowerPlacement` _asztd_instance)
    (if (`self.TowerActive`)
      (bind _currency (`/Game/ZTD_Blueprint/Blueprints/ZTD_Instance.Currency` _asztd_instance))
      ;[1 1 1] Towers that are already active are sold when clicked
      (set `/Game/ZTD_Blueprint/Blueprints/ZTD_Instance.Currency` (+ _currency 75) _asztd_instance)
      (`PrimitiveComponent.SetMaterial` (`self.TowerBody`) 0 "/Game/ZTD_Blueprint/Materials/TowerTransparent.TowerTransparent")
      (`PrimitiveComponent.SetMaterial` (`self.Sphere`) 0 "/Game/ZTD_Blueprint/Materials/TowerTransparent.TowerTransparent")
      (`PrimitiveComponent.SetMaterial` (`self.Cylinder`) 0 "/Game/ZTD_Blueprint/Materials/TowerTransparent.TowerTransparent")
      (set `self.TowerActive` false)
      (bind _outactors (`GameplayStatics.GetAllActorsOfClass` "/Game/ZTD_Blueprint/Blueprints/Tower_Tile.Tower_Tile_C"))
      (`/Game/ZTD_Blueprint/Blueprints/Tower_Tile.ChangeTower` _outactors)
      (else
        ;[1 1 1] If player has sufficient funds, a tower is purchased and activated
        (if (>= _currency 150)
          (set `/Game/ZTD_Blueprint/Blueprints/ZTD_Instance.Currency` (- _currency 150) _asztd_instance)
          (`PrimitiveComponent.SetMaterial` (`self.TowerBody`) 0 "/Game/ZTD_Blueprint/Materials/Tower.Tower")
          (`PrimitiveComponent.SetMaterial` (`self.Sphere`) 0 "/Game/ZTD_Blueprint/Materials/Tower.Tower")
          (`PrimitiveComponent.SetMaterial` (`self.Cylinder`) 0 "/Game/ZTD_Blueprint/Materials/Tower.Tower")
          (set `self.TowerActive` true)
          (else
            (`KismetSystemLibrary.PrintString` "Insufficient Funds!")))))))

(event `self.Sphere.OnClicked`
  (params (TouchedComponent :type "PrimitiveComponent Object Reference") (ButtonPressed :type "Key Structure" :default "AnyKey"))
  ;[1 1 1] When towers are purchased, they are set to a solid material and decrease currency. When sold they increase currency and set to transparent again
  (goto _label_2))

(event `self.Cylinder.OnClicked`
  (params (TouchedComponent :type "PrimitiveComponent Object Reference") (ButtonPressed :type "Key Structure" :default "AnyKey"))
  ;[1 1 1] When towers are purchased, they are set to a solid material and decrease currency. When sold they increase currency and set to transparent again
  (goto _label_2))

(fn `UserConstructionScript`)