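; Game mode for the ZTD game that runs a single small wave of zombies.
; While the wave is active, Tick uses a one-second Delay to call SpawnZombies, which creates a Zombie_Character at a fixed location and increments the spawn count.
; When Tick finds the count at its cap, it marks the wave complete.
; An unconnected chain would activate the wave on the ZTD_Instance game instance once a timer expires.
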(event `self.ReceiveTick`
  (params (DeltaSeconds :type "Float (single-precision)"))
  (if (`self.WaveActive`)
    (if (< (`self.WaveSpawned`) 3)
      (`KismetSystemLibrary.Delay` 1.0)
      (`self.SpawnZombies`)
      (else
        (set `self.WaveActive` false)
        (set `self.WaveComplete` true)))))

(event `SpawnZombies`
  (`KismetSystemLibrary.PrintString` "SpawningZombie" true true (struct :`G` 0.66 :`B` 1.0 :`A` 1.0) 1.0)
  (`|SpawnActorFromClass` "/Game/ZTD_Blueprint/Normal_Zombie_AI/Zombie_Character.Zombie_Character_C" (`KismetMathLibrary.MakeTransform` (4000.0 1900.0 222.0)) "Undefined" "OverrideRootScale")
  (set `self.WaveSpawned` (+ (`self.WaveSpawned`) 1)))

(fn `UserConstructionScript`)