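; Tower_Tile is an actor that acts as a clickable slot for placing a tower.
; Clicking an empty tile spawns a Test_Tower at the root transform, stores it and sets TowerExists to block further placement.
; Hover prints whether placement is possible, based on that flag.
; Ending hover always prints the "not placable" message, as it shares that print node regardless of state.
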(event `self.ReceiveTick`
  (params (DeltaSeconds :type "Float (single-precision)")))

(event `self.Tower_Tile.OnBeginCursorOver`
  (params (TouchedComponent :type "PrimitiveComponent Object Reference"))
  ;[1 1 1] Mousing over the tile shows that you can place a tower
  (if (`self.TowerExists`)
    (`KismetSystemLibrary.PrintString` "Tower is not Placable..." true true (struct :`G` 0.66 :`B` 1.0 :`A` 1.0) 1.0 :!label _label)
    (else
      (`KismetSystemLibrary.PrintString` "Tower is Placable!" true true (struct :`G` 0.66 :`B` 1.0 :`A` 1.0) 1.0))))

(event `self.Tower_Tile.OnEndCursorOver`
  (params (TouchedComponent :type "PrimitiveComponent Object Reference"))
  ;[1 1 1] Mousing over the tile shows that you can place a tower
  (goto _label))

(event `self.Tower_Tile.OnClicked`
  (params (TouchedComponent :type "PrimitiveComponent Object Reference") (ButtonPressed :type "Key Structure" :default "AnyKey"))
  ;[1 1 1] A tower actor is spawned when the player clicks the tile.
  (if (not (`self.TowerExists`))
    (bind _returnvalue (`|SpawnActorFromClass` "/Game/ZTD_Blueprint/Blueprints/Test_Tower.Test_Tower_C" (`SceneComponent.K2_GetComponentToWorld` (`self.DefaultSceneRoot`)) "Undefined" "OverrideRootScale"))
    (set `self.TowerA` _returnvalue)
    (set `self.TowerExists` true)))

(fn `UserConstructionScript`)