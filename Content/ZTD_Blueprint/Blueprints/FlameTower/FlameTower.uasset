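; Flamethrower tower for a zombie tower-defense game, bought and sold by clicking in placement mode.
; Clicking opens a purchase widget or sells an active tower; PurchaseTower charges currency, swaps materials and starts an attached flame effect.
; Tick updates visibility and overlaps; active towers turn toward the first overlapping zombie, applying AllFiredUp damage every frame.
; Overlap always sets ObjectsInRange true, so the idle spin runs only while inactive.
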(event `self.ReceiveBeginPlay`)

(event `self.ReceiveTick`
  (params (DeltaSeconds :type "Float (single-precision)"))
  ;[1 1 1] Tower Event Tick Flow
  (set `self.Delta Time` DeltaSeconds)
  (`self.TowerVisible`)
  (`self.Overlap`)
  (if (and (`self.ObjectsInRange`) (`self.TowerActive`))
    (`self.UpdateTurretRotation`)
    (else
      (`self.Idle`))))

(event `self.Tower1_Gun.OnClicked`
  (params (TouchedComponent :type "PrimitiveComponent Object Reference") (ButtonPressed :type "Key Structure" :default "AnyKey"))
  (bind _returnvalue (`GameplayStatics.GetPlayerController` 0))
  ;[1 1 1] When towers are purchased, they are set to a solid material and decrease currency. When sold they increase currency and set to transparent again
  (bind _asztd_instance (cast `/Game/ZTD_Blueprint/Blueprints/ZTD_Instance` (`GameplayStatics.GetGameInstance`) :!label _label))
  (if (not (`/Game/ZTD_Blueprint/Blueprints/ZTD_Instance.Is Over UI` _asztd_instance))
    (bind _asztd_instance_2 (cast `/Game/ZTD_Blueprint/Blueprints/ZTD_Instance` (`GameplayStatics.GetGameInstance`)))
    (if (`/Game/ZTD_Blueprint/Blueprints/ZTD_Instance.IsTowerPlacement` _asztd_instance_2)
      (if (`self.TowerActive`)
        ;[1 1 1] Towers that are already active are sold when clicked
        (set `/Game/ZTD_Blueprint/Blueprints/ZTD_Instance.Currency` (+ (`/Game/ZTD_Blueprint/Blueprints/ZTD_Instance.Currency` _asztd_instance_2) 75) _asztd_instance_2)
        (`PrimitiveComponent.SetMaterial` (`self.Tower1_Base`) 0 "/Game/ZTD_Blueprint/Materials/TowerTransparent.TowerTransparent")
        (`PrimitiveComponent.SetMaterial` (`self.Tower1_Gun`) 0 "/Game/ZTD_Blueprint/Materials/TowerTransparent.TowerTransparent")
        (set `self.TowerActive` false)
        (bind _outactors (`GameplayStatics.GetAllActorsOfClass` "/Game/ZTD_Blueprint/Blueprints/Tower_Tile.Tower_Tile_C"))
        (`/Game/ZTD_Blueprint/Blueprints/Tower_Tile.ChangeTower` _outactors)
        (`self.StopFiringh`)
        (else
          (bind _returnvalue_2 (`|CreateWidget` "/Game/ZTD_Blueprint/Blueprints/Game_UI/Confirm_purchase.Confirm_purchase_C"))
          (`WidgetBlueprintLibrary.SetInputMode_GameAndUIEx` _returnvalue _returnvalue_2 "DoNotLock" false)
          (`UserWidget.AddToViewport` _returnvalue_2 0)
          (set `PlayerController.bShowMouseCursor` true _returnvalue)
          (`GameplayStatics.SetGamePaused` true)
          (set `/Game/ZTD_Blueprint/Blueprints/Game_UI/Confirm_purchase.T_ID` self _returnvalue_2)
          (set `/Game/ZTD_Blueprint/Blueprints/Game_UI/Confirm_purchase.Towertype` 4 _returnvalue_2))))))

(event `TowerVisible`
  ;[1 1 1] Unpurchased towers are shown or hidden when in placement mode or shooting
  (bind _asztd_instance (cast `/Game/ZTD_Blueprint/Blueprints/ZTD_Instance` (`GameplayStatics.GetGameInstance`)))
  (if (`/Game/ZTD_Blueprint/Blueprints/ZTD_Instance.IsTowerPlacement` _asztd_instance)
    (`SceneComponent.SetVisibility` (`self.Tower1_Base`) true false :!label _label_2)
    (`SceneComponent.SetVisibility` (`self.Tower1_Gun`) true false)
    (elif (`self.TowerActive`)
      (goto _label_2)
      (else
        (`SceneComponent.SetVisibility` (`self.Tower1_Base`) false false)
        (`SceneComponent.SetVisibility` (`self.Tower1_Gun`) false false)))))

(event `self.Tower1_Base.OnClicked`
  (params (TouchedComponent :type "PrimitiveComponent Object Reference") (ButtonPressed :type "Key Structure" :default "AnyKey"))
  ;[1 1 1] When towers are purchased, they are set to a solid material and decrease currency. When sold they increase currency and set to transparent again
  (goto _label))

(event `Overlap`
  ;[1 1 1] New Detection for enemies in range
  (set `self.Current Targets` (`PrimitiveComponent.GetOverlappingActors` (`self.TriggerVolume`) "/Game/ZTD_Blueprint/Normal_Zombie_AI/Zombie_Character.Zombie_Character_C"))
  (set `self.ObjectsInRange` true))

(event `Fire Weapon`
  ;[1 1 1] Fire Gun
  (bind _asztd_instance (cast `/Game/ZTD_Blueprint/Blueprints/ZTD_Instance` (`GameplayStatics.GetGameInstance`)))
  (`GameplayStatics.PlaySound2D` "/Game/ZTD_Blueprint/Sounds/FLAMETHROWER.FLAMETHROWER" (`/Game/ZTD_Blueprint/Blueprints/ZTD_Instance.SoundLevel` _asztd_instance) (`KismetMathLibrary.RandomFloatInRange` 0.95 1.05))
  (`KismetSystemLibrary.Delay` (`self.Fire Interval`))
  (bind _returnvalue (`GameplayStatics.SpawnEmitterAttached` "/Game/ZTD_Blueprint/Blueprints/FlameTower/FireStuff.FireStuff" (`self.Tower1_Gun`) "Socket")))

(event `StopFiringh`
  (`ActorComponent.K2_DestroyComponent` (stale `Fire Weapon` _returnvalue)))

(event `Idle`
  (bind _returnvalue (`SceneComponent.K2_GetComponentRotation` (`self.Tower1_Gun`)))
  ;[1 1 1] Idle State
  (`SceneComponent.K2_SetWorldRotation` (`self.Tower1_Gun`) (`KismetMathLibrary.RInterpTo` _returnvalue (`KismetMathLibrary.MakeRotator` 0.0 0.0 (+ (.yaw _returnvalue) 5.0)) (`self.Delta Time`) (`self.Rotation Speed`)) false false))

(event `UpdateTurretRotation`
  (bind _item (`KismetArrayLibrary.Array_Get` (`self.Current Targets`)))
  ;[1 1 1] Turret Rotation
  (bind _aszombie_character (cast `/Game/ZTD_Blueprint/Normal_Zombie_AI/Zombie_Character` _item))
  (`/Game/ZTD_Blueprint/Normal_Zombie_AI/Zombie_Character.AllFiredUp` _aszombie_character (`self.Damage`))
  (`SceneComponent.K2_SetWorldRotation` (`self.Tower1_Gun`) (`KismetMathLibrary.RInterpTo` (`SceneComponent.K2_GetComponentRotation` (`self.Tower1_Gun`)) (`KismetMathLibrary.MakeRotator` 0.0 (.pitch (`KismetMathLibrary.FindLookAtRotation` (`SceneComponent.K2_GetComponentLocation` (`self.Tower1_Gun`)) (`self.K2_GetActorLocation` _item))) (.yaw (`KismetMathLibrary.FindLookAtRotation` (`SceneComponent.K2_GetComponentLocation` (`self.Tower1_Gun`)) (`self.K2_GetActorLocation` _item)))) (`self.Delta Time`) (`self.Rotation Speed`)) false false))

(fn `Purchase Tower`
  (params (A :type Integer))
  (if (>= A 400)
    (bind _asztd_instance (cast `/Game/ZTD_Blueprint/Blueprints/ZTD_Instance` (`GameplayStatics.GetGameInstance`)))
    (set `/Game/ZTD_Blueprint/Blueprints/ZTD_Instance.Currency` (- A 400) _asztd_instance)
    (`PrimitiveComponent.SetMaterial` (`self.Tower1_Base`) 0 "/Game/ZTD_Blueprint/Materials/Tower.Tower")
    (`PrimitiveComponent.SetMaterial` (`self.Tower1_Gun`) 0 "/Game/ZTD_Blueprint/Materials/Tower.Tower")
    (set `self.TowerActive` true)
    (`self.Fire Weapon`)
    (else
      (`KismetSystemLibrary.PrintString` "Insufficient Funds!"))))

(fn `UserConstructionScript`)