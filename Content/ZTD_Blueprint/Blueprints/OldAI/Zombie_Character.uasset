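; Old-AI zombie enemy character for a tower defense game that walks toward a goal and damages the Base on contact.
; Every Tick it updates its healthbar, refreshes Target from TriggerVolume overlaps, reissues AIMoveTo to the first entry and checks capsule overlaps for the end goal.
; Touching a Base deals damage and destroys the zombie.
; Lethal damage disables collision, awards game-instance Currency and unpossesses before delayed destruction; DetectPlayer is unused.
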(event OnComponentBeginOverlap(Capsule)
  (params (OverlappedComponent :type Primitive%20Component%20Object%20Reference) (OtherActor :type Actor%20Object%20Reference) (OtherComp :type Primitive%20Component%20Object%20Reference) (OtherBodyIndex :type Integer) (bFromSweep :type Boolean) (SweepResult :type Hit%20Result%20Structure%20%28by%20ref%29))
  ;[1 1 1] Check for base in range and then deal damage and despawn
  (bind _asbase (Utilities|Casting|CastToBase OtherActor))
  (Default|TakeDamage _asbase (Variables|Default|GetDamage))
  (Actor|DestroyActor))

(event Custom|Take%20Damage
  (params (BulletPower :type Float%20%28single-precision%29))
  (bind _output_get (Variables|Default|SetHealth (- (Variables|Default|GetHealth) BulletPower)))
  (if (<= _output_get 0.0)
    ;[1 1 1] Kills zombie and destroys the body after a second
    (CallFunction|KillZombie)
    (Utilities|FlowControl|Delay 1.0)
    (Actor|DestroyActor)))

(event Custom|MoveToTarget
  ;[1 1 1] Move to Actor (target)
  (AI|AIMoveTo self "0, 0, 0" (Utilities|Array|Get(acopy) (Variables|Default|GetTarget)) 5.0 false))

(event Custom|DetectBase
  ;[1 1 1] detect the end goal
  (bind _output_get (Variables|Default|SetTarget (Collision|GetOverlappingActors (Variables|Default|GetTriggerVolume) "/Game/ZTD_Blueprint/Blueprints/OldAI/Target.Target_C" :!class /Script/Engine.PrimitiveComponent)))
  (for _array_element _output_get
    _))

(event Custom|locationcheck
  ;[1 1 1] On Overlap, print end goal reached
  (bind _output_get (Variables|Default|SetTarget (Collision|GetOverlappingActors (Variables|Collision|GetCapsuleComponent) "/Game/ZTD_Blueprint/Blueprints/OldAI/Target.Target_C" :!class /Script/Engine.PrimitiveComponent)))
  (for _array_element _output_get
    (if (Utilities|Enum|Equal(Enum) "Target1189" (Utilities|GetDisplayName _array_element))
      (Development|PrintString "end goal reached"))))

(event Custom|DetectPlayer
  ;[1 1 1] UnUsed
  (bind _output_get (Variables|Default|SetTarget (Collision|GetOverlappingActors (Variables|Default|GetCapsule) "/Game/ZTD_Blueprint/Blueprints/OldAI/Target.Target_C" :!class /Script/Engine.PrimitiveComponent)))
  (for _array_element _output_get
    (bind _output_get_2 (Variables|Default|SetInRange (>= (Utilities|Array|Length (Variables|Default|GetTarget)) 1)))
    (if _output_get_2
      (Development|PrintString "player in range")
      (else
        (Development|PrintString "player not in range")))))

(event EventTick
  (params (DeltaSeconds :type Float%20%28single-precision%29))
  ;[1 1 1] Zombie Tick Flow
  (Variables|Default|SetDelta DeltaSeconds)
  (CallFunction|DrawHealthbar)
  (CallFunction|DetectBase)
  (CallFunction|MovetoTarget)
  (CallFunction|Locationcheck))

(fn ConstructionScript)

(fn KillZombie
  (Collision|SetActorEnableCollision false)
  (bind _asztd_instance (Utilities|Casting|CastToZTD_Instance (Game|GetGameInstance)))
  (Variables|/Game/ZTD_Blueprint/Blueprints/ZTD_Instance.ZTD_Instance_C|SetCurrency _asztd_instance (+ (Variables|/Game/ZTD_Blueprint/Blueprints/ZTD_Instance.ZTD_Instance_C|GetCurrency _asztd_instance) 100))
  (bind _returnvalue (AI|GetAIController self))
  (Pawn|UnPossess _returnvalue))

(fn DrawHealthbar
  (bind _aszombie_healthbar (Utilities|Casting|CastToZombieHealthbar (UserInterface|GetUserWidgetObject (Variables|Default|Gethealthbar))))
  (Variables|/Game/ZTD_Blueprint/Blueprints/HUD/ZombieHealthbar.ZombieHealthbar_C|SetZombieHealth _aszombie_healthbar (Variables|Default|GetHealth)))

(fn ReturnBaseHealth
  (return (stale _health)))