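; AI controller for zombies that starts their behavior tree on possession.
; On possess, it casts the pawn to Zombie_Character, calls DetectBase on it, then runs AI_Behavior.
; AI perception updates for Player_Character only print debug messages when the player is sensed or lost.
; Unconnected leftover logic holds a sphere-plus-line-trace range check and a CanSeePlayer blackboard write, neither of which executes.
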(event `self.OnPossess`
  (params (PossessedPawn :type "Pawn Object Reference"))
  ;[1 1 1] Run Behavior Tree And sight perception Activation
  (bind _aszombie_character (cast `/Game/ZTD_Blueprint/Blueprints/OldAI/Zombie_Character` PossessedPawn))
  (`/Game/ZTD_Blueprint/Blueprints/OldAI/Zombie_Character.DetectBase` _aszombie_character)
  (`self.RunBehaviorTree` "/Game/ZTD_Blueprint/Blueprints/OldAI/AI_Behavior.AI_Behavior"))

(event `self.AIPerception.OnTargetPerceptionUpdated`
  (params (Actor :type "Actor Object Reference") (Stimulus :type "AIStimulus Structure"))
  ;[1 1 1] Run Behavior Tree And sight perception Activation
  (cast `/Game/ZTD_Blueprint/Blueprints/Player_Character` Actor)
  (if (`.bSuccessfullySensed` (break `AIStimulus` Stimulus))
    (`KismetSystemLibrary.PrintString` "Hello")
    (else
      (`KismetSystemLibrary.PrintString` "goodbye"))))

(fn `UserConstructionScript`)