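; Grenade actor for the grenade tower that deals area damage to zombies.
; On BeginPlay it waits half a second, gathers Zombie_Character actors overlapping AreaOfEffect, damages each and destroys itself.
; Unconnected logic would match the firing GrenadeTower by socket position and compute an arced launch velocity toward its first target, but it never runs.
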(event `GetStartLocation`
  ;[1 1 1] Finds inital Location and rotation and gets target location
  (set `self.Initial Location` (`SceneComponent.K2_GetComponentLocation` (`self.Sphere`))))

(event `ProjectilePath`
  ;[1 1 1] Finds Final Vel
  (bind _outlaunchvelocity (`GameplayStatics.SuggestProjectileVelocity_CustomArc` (`self.Initial Location`) (`self.TargetLocation`) 0.0 0.3))
  (set `self.FinalVelocity` _outlaunchvelocity))

(event `self.ReceiveBeginPlay`
  ;[1 1 1] Range of Bullet
  (cast `/Game/ZTD_Blueprint/Blueprints/ZTD_Instance` (`GameplayStatics.GetGameInstance`))
  (`KismetSystemLibrary.Delay` 0.5)
  (`self.Overlap`)
  (`self.Apply Damage`)
  (`self.K2_DestroyActor`))

(event `Overlap`
  ;[1 1 1] detect enemies in aoe
  (set `self.CurrentTargets` (`PrimitiveComponent.GetOverlappingActors` (`self.AreaOfEffect`) "/Game/ZTD_Blueprint/Blueprints/OldAI/Zombie_Character.Zombie_Character_C"))
  (bind _output_get (set `self.ObjectsInRange` (>= (`KismetArrayLibrary.Array_Length` (`self.CurrentTargets`)) 1)))
  (if _output_get
    (`KismetSystemLibrary.PrintString` "grenade- more than 0 zombies")
    (else
      (`KismetSystemLibrary.PrintString` "grenade - nothing in area"))))

(event `Apply Damage`
  ;[1 1 1] Apply Damage to all enemies in area
  (for _array_element (`self.CurrentTargets`)
    (bind _aszombie_character (cast `/Game/ZTD_Blueprint/Blueprints/OldAI/Zombie_Character` _array_element))
    (`/Game/ZTD_Blueprint/Blueprints/OldAI/Zombie_Character.Take Damage` _aszombie_character (`self.Damage`))))

(fn `UserConstructionScript`)