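; Grenade tower for the zombie tower defence game, bought or sold by clicking it during tower placement.
; Purchase goes through a paused confirmation widget; purchases and sales adjust GameInstance currency and swap solid or transparent materials.
; Tick hides inactive towers outside placement and polls the trigger volume for zombies.
; An active tower yaws toward the first target and spawns grenades, using Delay to throttle per-tick fire calls, otherwise it slowly spins.
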(event `self.ReceiveTick`
  (params (DeltaSeconds :type "Float (single-precision)"))
  ;[1 1 1] Tower Event Tick Flow
  (set `self.Delta Time` DeltaSeconds)
  (`self.SetTowerVisibility`)
  (`self.Overlap`)
  (if (and (`self.ObjectsInRange`) (`self.TowerActive`))
    (`self.UpdateTurretRotation`)
    (`self.Fire Weapon`)
    (else
      (`self.Idle`))))

(event `Visibility`
  (params (DeltaSeconds :type "Float (double-precision)" :default 0.0))
  (`self.SetTowerVisibility`))

(event `self.Tower1_Base.OnClicked`
  (params (TouchedComponent :type "PrimitiveComponent Object Reference") (ButtonPressed :type "Key Structure" :default "AnyKey"))
  (bind _returnvalue (`GameplayStatics.GetPlayerController` 0))
  ;[1 1 1] When towers are purchased, they are set to a solid material and decrease currency. When sold they increase currency and set to transparent again
  (bind _asztd_instance (cast `/Game/ZTD_Blueprint/Blueprints/ZTD_Instance` (`GameplayStatics.GetGameInstance`) :!label _label))
  (if (not (`/Game/ZTD_Blueprint/Blueprints/ZTD_Instance.Is Over UI` _asztd_instance))
    (bind _asztd_instance_2 (cast `/Game/ZTD_Blueprint/Blueprints/ZTD_Instance` (`GameplayStatics.GetGameInstance`)))
    (if (`/Game/ZTD_Blueprint/Blueprints/ZTD_Instance.IsTowerPlacement` _asztd_instance_2)
      (if (`self.TowerActive`)
        ;[1 1 1] Towers that are already active are sold when clicked
        (`self.SellTower` _asztd_instance_2 (`/Game/ZTD_Blueprint/Blueprints/ZTD_Instance.Currency` _asztd_instance_2))
        (else
          (bind _returnvalue_2 (`|CreateWidget` "/Game/ZTD_Blueprint/Blueprints/Game_UI/Confirm_purchase.Confirm_purchase_C"))
          (`WidgetBlueprintLibrary.SetInputMode_GameAndUIEx` _returnvalue _returnvalue_2 "DoNotLock" false)
          (`UserWidget.AddToViewport` _returnvalue_2 0)
          (set `PlayerController.bShowMouseCursor` true _returnvalue)
          (`GameplayStatics.SetGamePaused` true)
          (set `/Game/ZTD_Blueprint/Blueprints/Game_UI/Confirm_purchase.T_ID` self _returnvalue_2)
          (set `/Game/ZTD_Blueprint/Blueprints/Game_UI/Confirm_purchase.Towertype` 3 _returnvalue_2))))))

(event `self.Tower1_Gun.OnClicked`
  (params (TouchedComponent :type "PrimitiveComponent Object Reference") (ButtonPressed :type "Key Structure" :default "AnyKey"))
  ;[1 1 1] When towers are purchased, they are set to a solid material and decrease currency. When sold they increase currency and set to transparent again
  (goto _label))

(event `Fire Weapon`
  ;[1 1 1] Fire Gun
  (`KismetSystemLibrary.Delay` (`self.Fire Interval`))
  (`|SpawnActorFromClass` "/Game/ZTD_Blueprint/Blueprints/GrenadeTower/Grenade.Grenade_C" (`SceneComponent.GetSocketTransform` (`self.Tower1_Gun`) "Socket" "RTS_World") "Undefined" "OverrideRootScale"))

(event `Overlap`
  ;[1 1 1] New Detection for enemies in range
  (set `self.Current Targets` (`PrimitiveComponent.GetOverlappingActors` (`self.TriggerVolume`) "/Game/ZTD_Blueprint/Normal_Zombie_AI/Zombie_Character.Zombie_Character_C"))
  (bind _output_get (set `self.ObjectsInRange` (>= (`KismetArrayLibrary.Array_Length` (`self.Current Targets`)) 1))))

(event `Idle`
  (bind _returnvalue (`SceneComponent.K2_GetComponentRotation` (`self.Tower1_Gun`)))
  ;[1 1 1] Idle State
  (`SceneComponent.K2_SetWorldRotation` (`self.Tower1_Gun`) (`KismetMathLibrary.RInterpTo` _returnvalue (`KismetMathLibrary.MakeRotator` 0.0 0.0 (+ (.yaw _returnvalue) 5.0)) (`self.Delta Time`) (`self.Rotation Speed`)) false false))

(event `UpdateTurretRotation`
  ;[1 1 1] Turret Rotation
  (`SceneComponent.K2_SetWorldRotation` (`self.Tower1_Gun`) (`KismetMathLibrary.RInterpTo` (`SceneComponent.K2_GetComponentRotation` (`self.Tower1_Gun`)) (`KismetMathLibrary.MakeRotator` 0.0 0.0 (.yaw (`KismetMathLibrary.FindLookAtRotation` (`SceneComponent.K2_GetComponentLocation` (`self.Tower1_Gun`)) (`self.K2_GetActorLocation` (`KismetArrayLibrary.Array_Get` (`self.Current Targets`)))))) (`self.Delta Time`) (`self.Rotation Speed`)) false false))

(fn `PurchaseTower`
  (params (A :type Integer) (self2 :type "/Game/ZTD_Blueprint/Blueprints/ZTD_Instance Object Reference") (A2 :type Integer))
  (if (>= A 500)
    (bind _asztd_instance (cast `/Game/ZTD_Blueprint/Blueprints/ZTD_Instance` (`GameplayStatics.GetGameInstance`)))
    (set `/Game/ZTD_Blueprint/Blueprints/ZTD_Instance.Currency` (- A2 500) _asztd_instance)
    (`PrimitiveComponent.SetMaterial` (`self.Tower1_Base`) 0 "/Game/ZTD_Blueprint/Materials/Tower.Tower")
    (`PrimitiveComponent.SetMaterial` (`self.Tower1_Gun`) 0 "/Game/ZTD_Blueprint/Materials/Tower.Tower")
    (set `self.TowerActive` true)
    (else
      (`KismetSystemLibrary.PrintString` "Insufficient Funds!"))))

(fn `SellTower`
  (params (self2 :type "/Game/ZTD_Blueprint/Blueprints/ZTD_Instance Object Reference") (A :type Integer))
  (set `/Game/ZTD_Blueprint/Blueprints/ZTD_Instance.Currency` (+ A 125) self2)
  (`PrimitiveComponent.SetMaterial` (`self.Tower1_Base`) 0 "/Game/ZTD_Blueprint/Materials/TowerTransparent.TowerTransparent")
  (`PrimitiveComponent.SetMaterial` (`self.Tower1_Gun`) 0 "/Game/ZTD_Blueprint/Materials/TowerTransparent.TowerTransparent")
  (set `self.TowerActive` false)
  (bind _outactors (`GameplayStatics.GetAllActorsOfClass` "/Game/ZTD_Blueprint/Blueprints/Tower_Tile.Tower_Tile_C"))
  (`/Game/ZTD_Blueprint/Blueprints/Tower_Tile.ChangeTower` _outactors))

(fn `SetTowerVisibility`
  (bind _asztd_instance (cast `/Game/ZTD_Blueprint/Blueprints/ZTD_Instance` (`GameplayStatics.GetGameInstance`)))
  (if (`/Game/ZTD_Blueprint/Blueprints/ZTD_Instance.IsTowerPlacement` _asztd_instance)
    (`SceneComponent.SetVisibility` (`self.Tower1_Gun`) true false :!label _label)
    (`SceneComponent.SetVisibility` (`self.Tower1_Base`) true false)
    (elif (`self.TowerActive`)
      (goto _label)
      (else
        (`SceneComponent.SetVisibility` (`self.Tower1_Base`) false false)
        (`SceneComponent.SetVisibility` (`self.Tower1_Gun`) false false)))))

(fn `UserConstructionScript`)