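; Music actor, apparently for the game-over track, that plays its audio component at the volume stored in the game instance.
; BeginPlay sets the volume multiplier from the ZTD_Instance MusicLevel.
; An audio-finished event restarts GameoverMusic from the beginning and reapplies that volume, looping the track.
; Tick re-reads MusicLevel every frame to follow option changes, but only applies values above zero.
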(event `self.ReceiveActorBeginOverlap`
  (params (OtherActor :type "Actor Object Reference")))

(event `self.ReceiveBeginPlay`
  ;[1 1 1] Begin; pull sound from options
  (bind _asztd_instance (cast `/Game/ZTD_Blueprint/Blueprints/ZTD_Instance` (`GameplayStatics.GetGameInstance`) :!label _label))
  (`AudioComponent.SetVolumeMultiplier` (`self.Gameover_music`) (`/Game/ZTD_Blueprint/Blueprints/ZTD_Instance.MusicLevel` _asztd_instance)))

(event `self.Music3Audio.OnAudioFinished`
  ;[1 1 1] Loop as needed
  (`AudioComponent.Play` (`self.Gameover_music`) 0.0)
  (goto _label))

(event `self.ReceiveTick`
  (params (DeltaSeconds :type "Float (single-precision)"))
  ;[1 1 1] Adjust from options change
  (bind _asztd_instance (cast `/Game/ZTD_Blueprint/Blueprints/ZTD_Instance` (`GameplayStatics.GetGameInstance`))
    (:`then`
      _)
    (:`CastFailed`
      _))
  (bind _musiclevel (`/Game/ZTD_Blueprint/Blueprints/ZTD_Instance.MusicLevel` _asztd_instance))
  (if (> _musiclevel 0.0)
    (`AudioComponent.SetVolumeMultiplier` (`self.Gameover_music`) _musiclevel)))

(fn `UserConstructionScript`)